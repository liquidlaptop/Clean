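; Bomb trap actor that lights when hit by a BP_Lighter, then explodes and destroys itself.
; ActiveTrap and DeactivateTrap set the activation state and a HasChanged flag, which Tick polls and never resets.
; When active, Tick uses chained Delays to reveal particle, fire and explosion effects, then spawns and immediately destroys an Explosion1 actor before removing the bomb.
; When inactive, Tick hides those effects; DoIActivate is an empty stub.
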(event Custom|DeactivateTrap
  ;[1 1 1] Activate Deacivate Bomb
  (Rendering|SetVisibility (Variables|Default|GetParticleSystem) false false)
  (Variables|Default|SetIsTrapActivated false)
  (Variables|Default|SetHasChanged true))

(event Custom|Active%20Trap
  ;[1 1 1] Activate Deacivate Bomb
  (Rendering|SetVisibility (Variables|Default|GetParticleSystem) true false)
  (Variables|Default|SetIsTrapActivated true)
  (Variables|Default|SetHasChanged true))

(event EventTick
  (params (DeltaSeconds :type Float%20%28single-precision%29))
  ;[1 1 1] Has Bomb Status Changec
  (if (Variables|Default|GetHasChanged)
    (if (Variables|Default|GetIsTrapActivated)
      (Rendering|SetVisibility (Variables|Default|GetParticleSystem) true false)
      (Utilities|FlowControl|Delay 1.0)
      (Rendering|SetVisibility (Variables|Default|GetFire) true false)
      (Utilities|FlowControl|Delay 2.0)
      (Rendering|SetVisibility (Variables|Default|GetP_Explosion) true false)
      (Utilities|FlowControl|Delay 3.0)
      (bind _returnvalue (Game|SpawnActorfromClass "/Game/Assets_Dereks/DL_Explosions/Explosion1.Explosion1_C" (Transformation|GetWorldTransform (Variables|Default|GetStaticMeshComponent)) "Undefined" 0 0))
      (Actor|DestroyActor _returnvalue)
      (Transformation|SetWorldTransform (Variables|Default|GetStaticMeshComponent) (Math|Transform|MakeTransform "782.000000,2487.000000,251.000000" "0, 0,-90.000000" "0.200000,0.200000,0.200000") false false)
      (Actor|DestroyActor)
      (else
        (Rendering|SetVisibility (Variables|Default|GetParticleSystem) false false)
        (Rendering|SetVisibility (Variables|Default|GetFire) false false)
        (Rendering|SetVisibility (Variables|Default|GetP_Explosion) false false)))))

(event Collision|EventHit
  (params (MyComp :type Primitive%20Component%20Object%20Reference) (Other :type Actor%20Object%20Reference) (OtherComp :type Primitive%20Component%20Object%20Reference) (bSelfMoved :type Boolean) (HitLocation :type Vector :default "0, 0, 0") (HitNormal :type Vector :default "0, 0, 0") (NormalImpulse :type Vector :default "0, 0, 0") (Hit :type Hit%20Result%20Structure%20%28by%20ref%29))
  ;[1 1 1] Bomb Touches a Lights so Activates
  (if (== (Utilities|GetClass (.HitActor (Collision|BreakHitResult Hit))) "/Game/Assets_Dereks/DL_Assets/DL_Traps/BP_Lighter.BP_Lighter_C")
    (CallFunction|ActiveTrap)))

(fn ConstructionScript
  (|CallParentFunction))

(fn DoIActivate)