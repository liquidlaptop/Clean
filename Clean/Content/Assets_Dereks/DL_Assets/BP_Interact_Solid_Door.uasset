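; Door actor that toggles open and closed through a custom event, ignored while locked or already moving.
; The Moves flag selects sliding or rotating, with a timeline scaled by MoveX/Y/Z animating DefaultMesh's relative transform and reversing to close.
; Tick copies DefaultMesh's world transform onto StaticMeshdoor whenever they differ.
; Separate custom events lock, unlock or toggle the lock.
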(event Custom|CustomEvent
  (if (not (Variables|Default|GetIsLocked?))
    (if (not (Variables|Default|GetIsMoving))
      (Variables|Default|SetIsMoving true)
      (if (Variables|Default|GetMoves?)
        (if (Variables|Default|GetClosed?)
          (Variables|Default|SetClosed? false)
          (bind _newtrack_0 (Timeline|Timeline_1 PlayFromStart)
            (:Update
              (Transformation|SetRelativeLocation (Variables|Default|GetDefaultMesh) (Math|Vector|MakeVector (* _newtrack_0 (Variables|Default|GetMove%20X)) (* _newtrack_0 (Variables|Default|GetMove%20Y)) (* _newtrack_0 (Variables|Default|GetMove%20Z))) false false))
            (:Finished
              (Variables|Default|SetIsMoving false)))
          (else
            (Variables|Default|SetClosed? true)
            (Timeline|Timeline_1 ReverseFromEnd)))
        (elif (Variables|Default|GetClosed?)
          (Variables|Default|SetClosed? false)
          (bind _newtrack_0_2 (Timeline|Timeline_2 PlayFromStart)
            (:Update
              (Transformation|SetRelativeRotation (Variables|Default|GetDefaultMesh) (Math|Rotator|MakeRotator (* _newtrack_0_2 (Variables|Default|GetMove%20X)) (* _newtrack_0_2 (Variables|Default|GetMove%20Y)) (* _newtrack_0_2 (Variables|Default|GetMove%20Z))) false false))
            (:Finished
              (Variables|Default|SetIsMoving false)))
          (else
            (Variables|Default|SetClosed? true)
            (Timeline|Timeline_2 ReverseFromEnd)))))))

(event Custom|CustomEvent_1
  (Variables|Default|SetIsLocked? false))

(event Custom|CustomEvent_2
  (Variables|Default|SetIsLocked? true))

(event Custom|CustomEvent_3
  (if (Variables|Default|GetIsLocked?)
    (Variables|Default|SetIsLocked? false)
    (else
      (Variables|Default|SetIsLocked? true))))

(event EventBeginPlay)

(event Collision|EventActorBeginOverlap
  (params (OtherActor :type Actor%20Object%20Reference)))

(event EventTick
  (params (DeltaSeconds :type Float%20%28single-precision%29))
  (bind _defaultmesh (Variables|Default|GetDefaultMesh))
  (bind _staticmeshdoor (Variables|Default|GetStaticMeshdoor))
  (bind _returnvalue (Transformation|GetWorldTransform _defaultmesh))
  (if (not (== _returnvalue (Transformation|GetWorldTransform _staticmeshdoor)))
    (Transformation|SetWorldTransform _staticmeshdoor _returnvalue false false)))

(fn ConstructionScript
  (|CallParentFunction))