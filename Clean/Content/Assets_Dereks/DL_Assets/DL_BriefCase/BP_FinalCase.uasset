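; Grabbable briefcase that carries special pickup items in four socket slots while held.
; Tick detects changes in the grabbed state and swaps the visible lid, enabling physics-only collision on the held-state lid.
; On grab, overlapping items with code 2 attach to free sockets on CaseRep, tracked by a boolean slot array.
; On release, if items were taken, overlapping special items detach with physics enabled and the slots reset.
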(event EventBeginPlay)

(event Collision|EventActorBeginOverlap
  (params (OtherActor :type Actor%20Object%20Reference)))

(event EventTick
  (params (DeltaSeconds :type Float%20%28single-precision%29))
  (bind _lid2 (Variables|Default|GetLid2))
  (bind _lid2_2 (Variables|Default|GetLid2))
  (bind _caserep (Variables|Default|GetCaseRep))
  (bind _bp_pickupcudeisgrabbed_ (Variables|Default|GetBP_PickupCudeIsGrabbed?))
  (if (not (Math|Boolean|Equal(Boolean) (Variables|Default|GetLastGrab) (Variables|Default|GetBP_PickupCudeIsGrabbed?)))
    (Variables|Default|SetLastGrab _bp_pickupcudeisgrabbed_)
    (if _bp_pickupcudeisgrabbed_
      (Rendering|SetVisibility (Variables|Default|GetLid1) false false)
      (Rendering|SetVisibility _lid2 true false)
      (Collision|SetCollisionEnabled _lid2 "PhysicsOnly")
      (Collision|SetCollisionEnabled (Variables|Default|GetLid1) "NoCollision")
      (Development|PrintText "*Going to check for overlapping actors")
      (for _array_element (Collision|GetOverlappingActors (Variables|Default|GetBox) "/Game/Assets_Dereks/DL_Blueprints/BP_SpecialItems_Pickup.BP_SpecialItems_Pickup_C" :!class /Script/Engine.PrimitiveComponent)
        (bind _asbp_special_items_pickup (Utilities|Casting|CastToBP_SpecialItems_Pickup _array_element))
        (if (== (Variables|/Game/Assets_Dereks/DL_Blueprints/BP_SpecialItems_Pickup.BP_SpecialItems_Pickup_C|GetBP_PickupCudeItemCode _asbp_special_items_pickup) 2)
          (bind (_array_element_2 _array_index) (Utilities|Array|ForEachLoopwithBreak (Variables|Default|GetSlots) :!label _label)
            (:LoopBody
              (if (not _array_element_2)
                (goto _label Break)))
            (:Completed
              (Utilities|Array|SetArrayElem (Variables|Default|GetSlots) _array_index true)
              (switch int _array_index
                (:0
                  (Transformation|AttachComponentToComponent _array_element _caserep "Slot1" "SnapToTarget" "SnapToTarget" "KeepWorld" true)
                  (Utilities|Array|SetArrayElem (Variables|Default|GetSlots) 0 true))
                (:1
                  (Transformation|AttachComponentToComponent _array_element _caserep "Slot2" "SnapToTarget" "SnapToTarget" "KeepWorld" true)
                  (Utilities|Array|SetArrayElem (Variables|Default|GetSlots) 1 true))
                (:2
                  (Transformation|AttachComponentToComponent _array_element _caserep "Slot3" "SnapToTarget" "SnapToTarget" "KeepWorld" true)
                  (Utilities|Array|SetArrayElem (Variables|Default|GetSlots) 2 true))
                (:3
                  (Transformation|AttachComponentToComponent _array_element _caserep "Slot4" "SnapToTarget" "SnapToTarget" "KeepWorld" true)
                  (Utilities|Array|SetArrayElem (Variables|Default|GetSlots) 3 true)))
              (Variables|Default|SetGotItems true)))))
      (else
        (Rendering|SetVisibility (Variables|Default|GetLid1) true false)
        (Rendering|SetVisibility _lid2_2 false false)
        (Collision|SetCollisionEnabled _lid2_2 "NoCollision")
        (Collision|SetCollisionEnabled (Variables|Default|GetLid1) "NoCollision")
        (if (Variables|Default|GetGotItems)
          (for _array_element_3 (Collision|GetOverlappingActors (Variables|Default|GetBox) "/Game/Assets_Dereks/DL_Blueprints/BP_SpecialItems_Pickup.BP_SpecialItems_Pickup_C" :!class /Script/Engine.PrimitiveComponent)
            (bind _asbp_special_items_pickup_2 (Utilities|Casting|CastToBP_SpecialItems_Pickup _array_element_3))
            (Transformation|DetachFromActor _asbp_special_items_pickup_2 "KeepWorld" "KeepWorld" "KeepWorld")
            (Physics|SetSimulatePhysics (Variables|/Script/Engine.StaticMeshActor|GetStaticMeshComponent _asbp_special_items_pickup_2) true)
            (CallFunction|OutputSlotStatus))
          (Variables|Default|SetSlots (Variables|Default|GetEmptySlots)))))))

(event Collision|EventActorEndOverlap
  (params (OtherActor :type Actor%20Object%20Reference)))

(fn ConstructionScript
  (|CallParentFunction))

(fn OutputSlotStatus
  (for (_array_element _array_index) (Variables|Default|GetSlots)
    (Development|PrintText (Utilities|Text|FormatText "*Slot {0} Is {1}" _array_index (Utilities|Text|ToText(Boolean) _array_element)))))