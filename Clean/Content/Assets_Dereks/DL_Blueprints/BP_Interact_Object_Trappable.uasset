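; An interactable object, apparently a drawer, that can hide a bomb trap.
; A non-activated BP_Trap_Bomb hitting it while open is destroyed and stored as an armed trap, then InteractWithObject is called.
; Tick uses a HasChanged flag to update trap mesh and particle visibility.
; Once the object is open and stationary, Tick clears any stored trap and spawns a bomb above it with the same activation state.
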(event EventTick
  (params (DeltaSeconds :type Float%20%28single-precision%29))
  (bind _staticmesh (Variables|Default|GetStaticMesh))
  ;[1 1 1] Update the Display
  (if (Variables|Default|GetHasChanged?)
    (Variables|Default|SetHasChanged? false)
    (if (Variables|Default|GetHasTrap?)
      (Rendering|SetVisibility _staticmesh true false)
      (if (Variables|Default|GetTrapActivated?)
        (Rendering|SetVisibility (Variables|Default|GetParticleSystem) true false)
        (else
          (Rendering|SetVisibility (Variables|Default|GetParticleSystem) false false)))
      (else
        (Rendering|SetVisibility _staticmesh false false)))
    (elif (not (Variables|Default|GetClosed?))
      (if (not (Variables|Default|GetIsMoving))
        (if (Variables|Default|GetHasTrap?)
          (if (Variables|Default|GetTrapActivated?)
            (Variables|Default|SetHasTrap? false)
            (Variables|Default|SetTrapActivated? false)
            (Variables|Default|SetHasChanged? true)
            (CallFunction|ProduceTrapinWorld true)
            (else
              (Variables|Default|SetHasTrap? false)
              (Variables|Default|SetTrapActivated? false)
              (Variables|Default|SetHasChanged? true)
              (CallFunction|ProduceTrapinWorld false))))))))

(event Collision|EventHit
  (params (MyComp :type Primitive%20Component%20Object%20Reference) (Other :type Actor%20Object%20Reference) (OtherComp :type Primitive%20Component%20Object%20Reference) (bSelfMoved :type Boolean) (HitLocation :type Vector :default "0, 0, 0") (HitNormal :type Vector :default "0, 0, 0") (NormalImpulse :type Vector :default "0, 0, 0") (Hit :type Hit%20Result%20Structure%20%28by%20ref%29))
  (bind _hitactor (Collision|BreakHitResult Hit))
  ;[1 1 1] Bomb Dropped into Draw?
  (if (not (Variables|Default|GetClosed?))
    (if (== (Utilities|GetClass _hitactor) "/Game/Assets_Dereks/DL_Assets/DL_Traps/BP_Trap_Bomb.BP_Trap_Bomb_C")
      (if (not (Variables|Default|GetHasTrap?))
        (bind _asbp_trap_bomb (Utilities|Casting|CastToBP_Trap_Bomb _hitactor))
        (if (not (Variables|/Game/Assets_Dereks/DL_Assets/DL_Traps/BP_Trap_Bomb.BP_Trap_Bomb_C|GetIsTrapActivated _asbp_trap_bomb))
          (Variables|Default|SetTrapActivated? true)
          (Variables|Default|SetHasTrap? true)
          (Variables|Default|SetHasChanged? true)
          (Actor|DestroyActor _hitactor)
          (CallFunction|InteractwithObject))))))

(fn ConstructionScript
  (|CallParentFunction))

(fn ProduceTrapinWorld
  (params (TrapActivated :type Boolean))
  (bind _defaultsceneroot (Variables|Default|GetDefaultSceneRoot))
  (bind _returnvalue (Transformation|GetWorldTransform _defaultsceneroot))
  (bind _returnvalue_2 (Game|SpawnActorfromClass "/Game/Assets_Dereks/DL_Assets/DL_Traps/BP_Trap_Bomb.BP_Trap_Bomb_C" (Math|Transform|MakeTransform (Math|Vector|MakeVector (- (.x (.location _returnvalue)) 0.0) (+ (.y (.location _returnvalue)) -3e+01) (+ (.z (.location _returnvalue)) 1e+02)) (.rotation _returnvalue) (* (.scale _returnvalue) 0.6)) "Undefined" 0 true 0))
  (Variables|/Game/Assets_Dereks/DL_Assets/DL_Traps/BP_Trap_Bomb.BP_Trap_Bomb_C|SetIsTrapActivated _returnvalue_2 TrapActivated)
  (Variables|/Game/Assets_Dereks/DL_Assets/DL_Traps/BP_Trap_Bomb.BP_Trap_Bomb_C|SetHasChanged _returnvalue_2 true))