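; Level-start item randomizer that relocates already-placed pickups to random BP_Item_Spawn points.
; On BeginPlay it gathers those points, moves key pickups (item code 2) first, then BP_FinalCase actors, shrinking the pool after each.
; Each random index is rolled separately for move and removal, so the removed point may differ from the used one.
; Weapon and remaining-item passes are unconnected copies of the briefcase loop.
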(event EventBeginPlay
  (Development|PrintText "*Level Start Spawn Items")
  (bind _outactors (Actor|GetAllActorsOfClass "/Game/Assets_Dereks/DL_Blueprints/BP_Item_Spawn.BP_Item_Spawn_C"))
  (bind _output_get (Variables|Default|SetAvailableSpawnPointsItems _outactors))
  (bind _output_get_2 (Variables|Default|SetAvailableSpawnPointsItemsTemp _output_get))
  (bind _output_get_3 (Variables|Default|SetNumberSpawnPoints (Utilities|Array|Length _output_get_2)))
  (Variables|Default|SetNumberSpawnPointsRemaining _output_get_3)
  (bind _outactors_2 (Actor|GetAllActorsOfClass "/Game/Assets_Dereks/DL_Blueprints/BP_SpecialItems_Pickup.BP_SpecialItems_Pickup_C"))
  (for _array_element _outactors_2
    ;[1 1 1] Spawn The Keys First
    (if (== (Variables|/Game/Assets_Dereks/DL_Blueprints/BP_SpecialItems_Pickup.BP_SpecialItems_Pickup_C|GetBP_PickupCudeItemCode _array_element) 2)
      (Transformation|SetActorLocation _array_element (Transformation|GetActorLocation (Utilities|Array|Get(acopy) (Variables|Default|GetAvailableSpawnPointsItems) (Math|Random|RandomInteger (Variables|Default|GetNumberSpawnPointsRemaining)))) false false)
      (Utilities|Array|RemoveIndex (Variables|Default|GetAvailableSpawnPointsItems) (Math|Random|RandomInteger (Variables|Default|GetNumberSpawnPointsRemaining)))
      (Variables|Default|SetNumberSpawnPointsRemaining (- (Variables|Default|GetNumberSpawnPointsRemaining) 1))))
  (bind _outactors_3 (Actor|GetAllActorsOfClass "/Game/Assets_Dereks/DL_Assets/DL_BriefCase/BP_FinalCase.BP_FinalCase_C"))
  (for _array_element_2 _outactors_3
    ;[1 1 1] Spawn The Brief Case
    (Transformation|SetActorLocation _array_element_2 (Transformation|GetActorLocation (Utilities|Array|Get(acopy) (Variables|Default|GetAvailableSpawnPointsItems) (Math|Random|RandomInteger (Variables|Default|GetNumberSpawnPointsRemaining)))) false false)
    (Utilities|Array|RemoveItem (Variables|Default|GetAvailableSpawnPointsItems) (Utilities|Array|Get(acopy) (Variables|Default|GetAvailableSpawnPointsItems) (Math|Random|RandomInteger (Variables|Default|GetNumberSpawnPointsRemaining))))
    (Variables|Default|SetNumberSpawnPointsRemaining (- (Variables|Default|GetNumberSpawnPointsRemaining) 1))))

(fn ConstructionScript)