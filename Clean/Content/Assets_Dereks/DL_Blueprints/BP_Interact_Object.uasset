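; BP_Interact_Object is a configurable interactable serving as a door, moving object or door lock, with a swappable, scalable mesh.
; Interacting toggles it open or closed, using timelines to slide or rotate the mesh by per-axis amounts.
; Locked objects check overlapping locks with matching codes; an open lock unlocks them, then may attach or vanish, otherwise a sound plays.
; A lock that finishes closing locks overlapping closed objects sharing its code.
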(event Custom|Interact_With_Object
  ;[1 1 1] Actual Interaction
  (Development|PrintText (Variables|Default|GetIAm))
  (if (Variables|Adjusters_Locks|GetIsLocked?)
    ;[1 1 1] Comment
    (bind _array_element (Utilities|Array|ForEachLoopwithBreak (Collision|GetOverlappingActors (Variables|Default|GetBox) "BP_Interact_Object_C" :!class /Script/Engine.PrimitiveComponent))
      (:LoopBody
        (bind _asbp_interact_object (Utilities|Casting|CastToBP_Interact_Object _array_element))
        (if (Variables|BP_Interact_Object_C|GetIsDoorLock _asbp_interact_object)
          (if (== (Variables|BP_Interact_Object_C|GetDoorLockCode _asbp_interact_object) (Variables|Adjusters_Locks|GetDoorLockCode))
            (if (Variables|BP_Interact_Object_C|GetClosed? _asbp_interact_object)
              (Variables|Adjusters_Locks|SetIsLocked? true)
              (else
                (Variables|Adjusters_Locks|SetIsLocked? false)
                (Development|PrintText (Utilities|Text|FormatText "*I AM {0} and {2}  He is {1} and Moves with door {3}" (Variables|Default|GetIAm) (Utilities|Text|ToText(Boolean) (Variables|Adjusters_Locks|GetIsLocked?)) (Variables|BP_Interact_Object_C|GetIAm _asbp_interact_object) (Utilities|Text|ToText(Boolean) (Variables|BP_Interact_Object_C|GetDoesKeyMoveWithDoor _asbp_interact_object))))
                (if (Variables|BP_Interact_Object_C|GetDoesKeyMoveWithDoor _asbp_interact_object)
                  (Development|PrintText "*Attaching Door lock to me socket")
                  (Transformation|AttachComponentToComponent _asbp_interact_object (Variables|Default|GetDefaultMesh) "Socket" "KeepRelative" "KeepRelative" "KeepRelative" true)
                  (elif (Variables|BP_Interact_Object_C|GetDoesKeyVanishWithUnlock _asbp_interact_object)
                    (Actor|DestroyActor _asbp_interact_object))))))))
      (:Completed
        (if (Variables|Adjusters_Locks|GetIsLocked?)
          (Audio|SpawnSound2D "/Game/Assets_Dereks/DL_Assets/DL_Sounds/door-lock-1.door-lock-1")
          (else
            (if (not (Variables|AdjustersMovement|GetIsMoving)) :!label _label
              (Variables|AdjustersMovement|SetIsMoving true)
              (if (Variables|AdjustersMovement|GetMoves?)
                (if (Variables|AdjustersMovement|GetClosed?)
                  (Variables|AdjustersMovement|SetClosed? false)
                  (bind _newtrack_0 (Timeline|BlendOpenClose PlayFromStart)
                    (:Update
                      (Transformation|SetRelativeLocation (Variables|Default|GetDefaultMesh) (Math|Vector|MakeVector (* _newtrack_0 (Variables|AdjustersMovement|GetMove%20X)) (* _newtrack_0 (Variables|AdjustersMovement|GetMove%20Y)) (* _newtrack_0 (Variables|AdjustersMovement|GetMove%20Z))) false false))
                    (:Finished
                      (Variables|AdjustersMovement|SetIsMoving false)
                      ;[1 1 1] If Iam a Lock, see if I'm touching any Objects with same doorlockcode
                      (if (Variables|Adjusters_Locks|GetIsDoorLock) :!label _label_2
                        (for _array_element_2 (Collision|GetOverlappingActors (Variables|Default|GetBox) "BP_Interact_Object_C" :!class /Script/Engine.PrimitiveComponent)
                          (bind _asbp_interact_object_2 (Utilities|Casting|CastToBP_Interact_Object _array_element_2))
                          (if (not (Variables|BP_Interact_Object_C|GetIsDoorLock _asbp_interact_object_2))
                            (if (== (Variables|BP_Interact_Object_C|GetDoorLockCode _asbp_interact_object_2) (Variables|Adjusters_Locks|GetDoorLockCode))
                              (if (Variables|AdjustersMovement|GetClosed?)
                                (if (Variables|BP_Interact_Object_C|GetClosed? _asbp_interact_object_2)
                                  (CallFunction|LockDoor _asbp_interact_object_2)))))))))
                  (else
                    (Variables|AdjustersMovement|SetClosed? true)
                    (Timeline|BlendOpenClose ReverseFromEnd)))
                (elif (Variables|AdjustersMovement|GetClosed?)
                  (Variables|AdjustersMovement|SetClosed? false)
                  (bind _newtrack_0_2 (Timeline|Timeline_0 PlayFromStart)
                    (:Update
                      (Transformation|SetRelativeRotation (Variables|Default|GetDefaultMesh) (Math|Rotator|MakeRotator (* _newtrack_0_2 (Variables|AdjustersMovement|GetMove%20X)) (* _newtrack_0_2 (Variables|AdjustersMovement|GetMove%20Y)) (* _newtrack_0_2 (Variables|AdjustersMovement|GetMove%20Z))) false false))
                    (:Finished
                      (Variables|AdjustersMovement|SetIsMoving false)
                      (goto _label_2)))
                  (else
                    (Variables|AdjustersMovement|SetClosed? true)
                    (Timeline|Timeline_0 ReverseFromEnd)))))))))
    (else
      (goto _label))))

(event Custom|Unlock_Door
  ;[1 1 1] Lock / Unlock Door
  (bind _output_get (Variables|Adjusters_Locks|SetIsLocked? false))
  (Development|PrintText (Utilities|Text|FormatText "* {0} Locked? {1}" (Variables|Default|GetIAm) (Utilities|Text|ToText(Integer) 0 _output_get))))

(event Custom|Lock_Door
  ;[1 1 1] Lock / Unlock Door
  (Variables|Adjusters_Locks|SetIsLocked? true)
  (Development|PrintText (Utilities|Text|FormatText "* {0} Locked? {1}" (Variables|Default|GetIAm) (Utilities|Text|ToText(Integer) 0 (stale Custom|Unlock_Door _output_get)))))

(event Custom|Lock_Toggle
  ;[1 1 1] Lock / Unlock Door
  (if (Variables|Adjusters_Locks|GetIsLocked?)
    (bind _output_get (Variables|Adjusters_Locks|SetIsLocked? false))
    (else
      (Variables|Adjusters_Locks|SetIsLocked? true)))
  (Development|PrintText (Utilities|Text|FormatText "* {0} Locked? {1}" (Variables|Default|GetIAm) (Utilities|Text|ToText(Integer) 0 _output_get))))

(fn ConstructionScript
  (bind _meshscale (Variables|Default|GetMeshScale))
  (bind _object_mesh (Variables|Default|GetObject_Mesh))
  ;[1 1 1] Construction Script Swappedable Mesh
  (Transformation|SetRelativeScale3D (Variables|Default|GetDefaultMesh) (Math|Vector|MakeVector _meshscale _meshscale _meshscale))
  (if (!= _object_mesh 0)
    (Components|StaticMesh|SetStaticMesh (Variables|Default|GetDefaultMesh) _object_mesh)))