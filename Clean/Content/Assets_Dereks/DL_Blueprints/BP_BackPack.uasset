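; Backpack actor that stores grabbed pickups as item codes in a size-limited inventory and ejects them when hit.
; On overlap, it scans the other actor's attached actors for grabbed, backpackable BP_Prob_Pickups, records their codes and destroys them.
; Ejection handles only the first entry, spawning a key above the pack for code 1; otherwise its busy flag stays set.
; The construction script applies a configurable mesh and scale.
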(event Custom|Eject_Items
  (bind _defaultsceneroot (Variables|Default|GetDefaultSceneRoot))
  (bind _inventory_id (Variables|Default|GetInventory_id))
  (bind _item (Utilities|Array|Get(acopy) _inventory_id))
  (bind _returnvalue (Transformation|GetWorldTransform _defaultsceneroot))
  ;[1 1 1] Eject All Items
  (if (not (Variables|Default|GetAmIEjecting?))
    (Variables|Default|SetAmIEjecting? true)
    (Development|PrintText "*BackPack I been Hit")
    (if (> (Utilities|Array|Length (Variables|Default|GetInventory_id)) 0)
      (Development|PrintText (Utilities|Text|FormatText "*{0} NUmber spawn" _item))
      (switch int _item
        (:1
          (Development|PrintText "*Trying to Spawn??")
          (Utilities|Array|RemoveIndex (Variables|Default|GetInventory_id))
          (Game|SpawnActorfromClass "/Game/Assets_Dereks/DL_Assets/DL_Props/Item1_Key.Item1_Key_C" (Math|Transform|MakeTransform (Math|Vector|MakeVector (.x (.location _returnvalue)) (+ (.y (.location _returnvalue)) 0.0) (+ (.z (.location _returnvalue)) 1e+02 (Math|Conversions|ToFloat(Integer) (Math|Random|RandomInteger 50)))) (.rotation _returnvalue) "0.500000,0.500000,0.500000") "AlwaysSpawn" 0 false false 0 false "(R=0.000000,G=0.000000,B=0.000000,A=0.000000)" "" 0.0)
          (Development|PrintText "*Produceds Item???")
          (Variables|Default|SetAmIEjecting? false)
          (CallFunction|HowManyItemsIGot "*"))))))

(event Collision|EventHit
  (params (MyComp :type Primitive%20Component%20Object%20Reference) (Other :type Actor%20Object%20Reference) (OtherComp :type Primitive%20Component%20Object%20Reference) (bSelfMoved :type Boolean) (HitLocation :type Vector :default "0, 0, 0") (HitNormal :type Vector :default "0, 0, 0") (NormalImpulse :type Vector :default "0, 0, 0") (Hit :type Hit%20Result%20Structure%20%28by%20ref%29))
  (CallFunction|EjectItems))

(event Collision|EventActorBeginOverlap
  (params (OtherActor :type Actor%20Object%20Reference))
  (bind _inventory_id (Variables|Default|GetInventory_id))
  ;[1 1 1] Put Items In BackPck
  (for _array_element (Actor|GetAttachedActors OtherActor)
    (if (== (Utilities|GetClass _array_element) "/Game/Assets_Dereks/DL_Blueprints/BP_Prob_Pickup.BP_Prob_Pickup_C")
      (bind _asbp_prob_pickup (Utilities|Casting|CastToBP_Prob_Pickup _array_element))
      (if (Variables|/Game/Assets_Dereks/DL_Blueprints/BP_Prob_Pickup.BP_Prob_Pickup_C|GetBP_PickupCudeIsGrabbed? _asbp_prob_pickup)
        (if (Variables|/Game/Assets_Dereks/DL_Blueprints/BP_Prob_Pickup.BP_Prob_Pickup_C|GetBP_PickupCubeIsBackPackable? _asbp_prob_pickup)
          (if (< (Utilities|Array|Length _inventory_id) (Variables|Default|GetInventorySize))
            (Utilities|Array|Add _inventory_id (Variables|/Game/Assets_Dereks/DL_Blueprints/BP_Prob_Pickup.BP_Prob_Pickup_C|GetBP_PickupCudeItemCode _asbp_prob_pickup))
            (CallFunction|HowManyItemsIGot "*")
            (Actor|DestroyActor _array_element))))))
  (Development|PrintText "*Finished Childs"))

(fn ConstructionScript
  (bind _objectmesh (Variables|Default|GetObjectMesh))
  (bind _meshscale (Variables|Default|GetMeshScale))
  ;[1 1 1] Construction Script Swappedable Mesh
  (Transformation|SetRelativeScale3D (Variables|Default|GetDefaultMesh) (Math|Vector|MakeVector _meshscale _meshscale _meshscale))
  (if (!= _objectmesh 0)
    (Components|StaticMesh|SetStaticMesh (Variables|Default|GetDefaultMesh) _objectmesh)))

(fn HowManyItemsIGot
  (params (text :type Text))
  (bind _inventorysize (Variables|Default|GetInventorySize))
  (bind _inventory_id (Variables|Default|GetInventory_id))
  (bind _returnvalue (Utilities|Array|Length _inventory_id))
  (Development|PrintText (Utilities|Text|FormatText "*{5} I Have {0} Items out of {1} Leaving {2}" text _returnvalue _inventorysize (- _inventorysize _returnvalue))))